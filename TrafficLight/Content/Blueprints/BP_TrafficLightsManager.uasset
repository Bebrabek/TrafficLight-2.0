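; Traffic lights manager that runs an endless red, yellow, green cycle from BeginPlay.
; Recolor looks up each color in the ColorSettings map by enum key and passes it to ChangeColor on the first element of the matching light array.
; Fixed latent Delays time each phase, each light is set to black before the next, and the chain wires back on itself to repeat.
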(event `self.ReceiveBeginPlay`
  (`self.Recolor`))

(event `Recolor`
  (bind _output (`|GetArrayItem` (`self.LightRed`)))
  (bind _output_2 (`|GetArrayItem` (`self.LightYellow`)))
  (bind _output_3 (`|GetArrayItem` (`self.LightGreen`)))
  (bind _output_get (set `self.ColorSettings` (`self.ColorSettings`)))
  (`/Game/Blueprints/BP_TraffictLight.ChangeColor` _output (`BlueprintMapLibrary.Map_Find` (break `/Game/Blueprints/S_LIghtColor` _output_get) "NewEnumerator0") :!label _label)
  (`KismetSystemLibrary.Delay` 5.0)
  (`/Game/Blueprints/BP_TraffictLight.ChangeColor` :`self` _output)
  (`/Game/Blueprints/BP_TraffictLight1.ChangeColor` _output_2 (`BlueprintMapLibrary.Map_Find` (break `/Game/Blueprints/S_LIghtColor` _output_get) "NewEnumerator1"))
  (`KismetSystemLibrary.Delay` 2.0)
  (`/Game/Blueprints/BP_TraffictLight1.ChangeColor` :`self` _output_2)
  (`/Game/Blueprints/BP_TraffictLight2.ChangeColor` _output_3 (`BlueprintMapLibrary.Map_Find` (break `/Game/Blueprints/S_LIghtColor` _output_get) "NewEnumerator2"))
  (`KismetSystemLibrary.Delay` 3.0)
  (`/Game/Blueprints/BP_TraffictLight2.ChangeColor` :`self` _output_3)
  (goto _label))

(fn `UserConstructionScript`)